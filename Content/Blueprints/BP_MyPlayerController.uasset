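; Player controller that tracks progress fractions for four player abilities (MA, FA, SA, UA), covering cooldowns and ultimate-style charge.
; CooldownEvent zeroes MA, FA or SA by ability number and starts a looping timer at one-tenth of that ability's cooldown time from PlayerCharacter.
; Each timer adds a tenth per call, pausing only on an exact float match with 1.0.
; Tick sets UA from charging points divided by its UACC value.
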(event `self.ReceiveBeginPlay`
  (set `self.MAPercent` 1.0)
  (set `self.FAPercent` 1.0)
  (set `self.SAPercent` 1.0)
  (set `self.UAPercent` 1.0))

(event `self.ReceiveTick`
  (params (DeltaSeconds :type "Float (single-precision)"))
  (bind _asplayer_character (cast `PlayerCharacter` (`GameplayStatics.GetPlayerPawn` 0)))
  (set `self.UAPercent` (/ (`PlayerCharacter.GetChargingPoints` _asplayer_character) (`PlayerCharacter.GetUACC` _asplayer_character))))

(event `self.CooldownEvent`
  (params (Ability :type Integer))
  (bind _asplayer_character (cast `PlayerCharacter` (`GameplayStatics.GetPlayerPawn` 0)))
  (if (== Ability 1)
    (set `self.MAPercent` 0.0)
    (`KismetSystemLibrary.K2_SetTimer` null "AddMAPercent" (/ (`PlayerCharacter.GetMACT` _asplayer_character) 10.0) true)
    (elif (== Ability 2)
      (set `self.FAPercent` 0.0)
      (`KismetSystemLibrary.K2_SetTimer` null "AddFAPercent" (/ (`PlayerCharacter.GetFACT` _asplayer_character) 10.0) true)
      (elif (== Ability 3)
        (set `self.SAPercent` 0.0)
        (`KismetSystemLibrary.K2_SetTimer` null "AddSAPercent" (/ (`PlayerCharacter.GetSACT` _asplayer_character) 10.0) true)))))

(fn `AddFAPercent`
  (bind _asplayer_character (cast `PlayerCharacter` (`GameplayStatics.GetPlayerPawn` 0)))
  (bind _returnvalue (`PlayerCharacter.GetFACT` _asplayer_character))
  (bind _output_get (set `self.FAPercent` (+ (`self.FAPercent`) (/ (/ _returnvalue 10.0) _returnvalue))))
  (if (== _output_get 1.0)
    (`KismetSystemLibrary.K2_PauseTimer` null "AddFAPercent")))

(fn `AddMAPercent`
  (bind _asplayer_character (cast `PlayerCharacter` (`GameplayStatics.GetPlayerPawn` 0)))
  (bind _returnvalue (`PlayerCharacter.GetMACT` _asplayer_character))
  (bind _output_get (set `self.MAPercent` (+ (`self.MAPercent`) (/ (/ _returnvalue 10.0) _returnvalue))))
  (if (== _output_get 1.0)
    (`KismetSystemLibrary.K2_PauseTimer` null "AddMAPercent")))

(fn `AddSAPercent`
  (bind _asplayer_character (cast `PlayerCharacter` (`GameplayStatics.GetPlayerPawn` 0)))
  (bind _returnvalue (`PlayerCharacter.GetSACT` _asplayer_character))
  (bind _output_get (set `self.SAPercent` (+ (`self.SAPercent`) (/ (/ _returnvalue 10.0) _returnvalue))))
  (if (== _output_get 1.0)
    (`KismetSystemLibrary.K2_PauseTimer` null "AddSAPercent")))

(fn `UserConstructionScript`)